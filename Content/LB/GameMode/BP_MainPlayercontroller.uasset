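; Player controller that switches the player between the main pawn and other pawns, apparently for entering and leaving houses or rooms.
; Switching blends the view target, possesses the pawn, updates HouseStatus and fires the OnChangeHouseData dispatcher, with entry also notifying the main UI widget.
; SetHouseData stores house data and derives the status from whether its Mouse_L field is filled.
; AddPawn and FindPawn maintain a pawn registry searchable by ID.
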(event `self.ReceiveBeginPlay`
  (`KismetSystemLibrary.Delay` 0.2)
  (bind _foundwidgets (`WidgetBlueprintLibrary.GetAllWidgetsOfClass` "/Game/LB/UMG/WBP_MainUI.WBP_MainUI_C"))
  (set `self.MainUI` (`|GetArrayItem` _foundwidgets)))

(event `SetNewPawn`
  (params (NewPawn :type "Pawn Object Reference"))
  (`self.SetViewTargetWithBlend` NewPawn 3.0)
  (`self.Possess` NewPawn)
  (set `self.HouseStatus` "NewEnumerator1")
  (`/Game/LB/UMG/WBP_MainUI.Enter the room` (`self.MainUI`))
  (`self.OnChangeHouseData`))

(event `SetOldPawn`
  (bind _returnvalue (`GameplayStatics.GetActorOfClass` "/Game/LB/GameMode/BP_MainPawn.BP_MainPawn_C"))
  (`self.SetViewTargetWithBlend` _returnvalue 3.0)
  (`self.Possess` _returnvalue)
  (set `self.HouseStatus` "NewEnumerator0")
  (`self.OnChangeHouseData`))

(fn `AddPawn`
  (params (NewPawn :type "/Game/LB/BP/BP_WASD_Pawn Object Reference (by ref)"))
  (`KismetArrayLibrary.Array_AddUnique` (`self.Panws`) NewPawn))

(fn `FindPawn`
  (params (ID :type Text))
  (returns (NewParam :type "Pawn Object Reference"))
  (for _array_element (`self.Panws`)
    (if (`KismetTextLibrary.EqualEqual_TextText` (`/Game/LB/BP/BP_WASD_Pawn.ID` _array_element) ID)
      (return _array_element))))

(fn `SetHouseData`
  (params (HouseData :type "/Game/LB/Data/ST_HouseStruct Structure"))
  (bind _housedata_mouse_l (break `/Game/LB/Data/ST_HouseStruct` (`self.HouseData`)))
  (set `self.HouseData` HouseData)
  (if (not (`KismetStringLibrary.IsEmpty` _housedata_mouse_l))
    (set `self.HouseStatus` "NewEnumerator1")
    (return)
    (else
      (set `self.HouseStatus` "NewEnumerator0")
      (return))))

(fn `UserConstructionScript`)