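; BP_WASD_Pawn is a player pawn for moving around the level with WASD-style input and right-mouse look.
; On BeginPlay it registers itself with the player controller and adds the IMC_HousePawn Enhanced Input context.
; While right mouse is held, Tick turns mouse delta into actor yaw and clamped pitch.
; The move action drives half-scaled movement along the forward and right vectors, using only their horizontal components.
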(event `self.ReceiveBeginPlay`
  (`/Game/LB/GameMode/BP_MainPlayercontroller.AddPawn` (`/Game/LB/Communication/BPF_LB.Get My Player Controller`) self)
  (`EnhancedInputSubsystemInterface.AddMappingContext` (pcsubsystem `EnhancedInputLocalPlayerSubsystem` (`GameplayStatics.GetPlayerController` 0)) "/Game/LB/BP/IMC_HousePawn.IMC_HousePawn" 0 (struct)))

(event `Key|RightMouseButton`
  (params (Key :type "Key Structure"))
  (:`Pressed`
    (set `self.IsRotation` true))
  (:`Released`
    (set `self.IsRotation` false)))

(event `self.ReceiveTick`
  (params (DeltaSeconds :type "Float (single-precision)"))
  (bind (_returnvalue_roll _returnvalue_pitch _returnvalue_yaw) (`KismetMathLibrary.BreakRotator` (`self.K2_GetActorRotation`)))
  (bind (_deltax _deltay) (`PlayerController.GetInputMouseDelta` (`GameplayStatics.GetPlayerController` 0)))
  (if (`self.IsRotation`)
    (`self.K2_SetActorRotation` (`KismetMathLibrary.MakeRotator` 0.0 (`KismetMathLibrary.FClamp` (+ _deltay _returnvalue_pitch) -89.0 89.0) (+ _deltax _returnvalue_yaw)))))

(event `EnhancedInput|/Game/LB/BP/IA_HousePawn_Move`
  (params (ActionValue :type "Vector2D Structure") (ElapsedSeconds :type "Float (double-precision)") (TriggeredSeconds :type "Float (double-precision)") (InputAction :type "InputAction Object Reference" :default "/Game/LB/BP/IA_HousePawn_Move.IA_HousePawn_Move"))
  (bind (_returnvalue_x _returnvalue_y) (`KismetMathLibrary.BreakVector` (`self.GetActorForwardVector`)))
  (bind (_returnvalue_x_2 _returnvalue_y_2) (`KismetMathLibrary.BreakVector` (`self.GetActorRightVector`)))
  (:`Triggered`
    (`self.AddMovementInput` (`KismetMathLibrary.MakeVector` _returnvalue_x _returnvalue_y) (* ActionValue_X 0.5))
    (`self.AddMovementInput` (`KismetMathLibrary.MakeVector` _returnvalue_x_2 _returnvalue_y_2) (* ActionValue_Y -0.5))))

(fn `UserConstructionScript`)